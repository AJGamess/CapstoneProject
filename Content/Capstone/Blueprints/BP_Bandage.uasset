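; BP_Bandage is a usable healing item that restores the player's health.
; Its Use Item function increments the passed-in Player's Health by one when below MaxHealth and prints the new value.
; At full health it only prints a message that healing is not possible.
; The event graph and construction script add no logic of their own, and the item is not consumed here.
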(event EventBeginPlay
  (|CallParentFunction) ; This node is disabled and will not be called.\nDrag off pins to build functionality.
)

(event Collision|EventActorBeginOverlap
  (params (OtherActor :type Actor%20Object%20Reference))
  (|CallParentFunction OtherActor) ; This node is disabled and will not be called.\nDrag off pins to build functionality.
)

(event EventTick
  (params (DeltaSeconds :type Float%20%28single-precision%29))
  (|CallParentFunction DeltaSeconds) ; This node is disabled and will not be called.\nDrag off pins to build functionality.
)

(fn ConstructionScript
  (|CallParentFunction))

(fn UseItem
  (params (Player :type BP%20Player%20Character%20Object%20Reference))
  (bind _health (Variables|/Game/Capstone/Blueprints/BP_PlayerCharacter.BP_PlayerCharacter_C|GetHealth Player))
  (if (< _health (Variables|/Game/Capstone/Blueprints/BP_PlayerCharacter.BP_PlayerCharacter_C|GetMax%20Health Player))
    (bind _result (Math|Float|IncrementFloat _health)
      (:%20%20
        (Development|PrintString (Class|KismetStringLibrary|BuildStringDouble "Health at: " "" _result))))
    (else
      (Development|PrintString "Can't Heal. Already Full."))))