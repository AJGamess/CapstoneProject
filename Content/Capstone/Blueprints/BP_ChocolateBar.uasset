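; BP_ChocolateBar is a usable item that gives the player a temporary speed boost.
; Use Item fires Chocolate Boost, which tops up the sprint meter within a clamped range and scales walk and sprint speeds by StatusEffect.
; After a delay of TimeEffectIsActive, it restores both speeds to the player's defaults and destroys itself, so the actor lives until the effect ends.
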(event Custom|Chocolate%20Boost
  (params (Player :type BP%20Player%20Character%20Object%20Reference))
  (bind _status_effect (Variables|Default|GetStatus%20Effect))
  ;[0.15 0.15 0.15 0.5] Chocolate Boost
  (Variables|/Game/Capstone/Blueprints/BP_PlayerCharacter.BP_PlayerCharacter_C|SetSprint%20Meter Player (Math|Float|Clamp(Float) (+ (Variables|/Game/Capstone/Blueprints/BP_PlayerCharacter.BP_PlayerCharacter_C|GetSprint%20Meter Player) 0.5) 0.0 3.0))
  (Variables|/Game/Capstone/Blueprints/BP_PlayerCharacter.BP_PlayerCharacter_C|SetSprint%20Speed Player (* (Variables|/Game/Capstone/Blueprints/BP_PlayerCharacter.BP_PlayerCharacter_C|GetSprint%20Speed Player) _status_effect))
  (Variables|/Game/Capstone/Blueprints/BP_PlayerCharacter.BP_PlayerCharacter_C|SetWalk%20Speed Player (* (Variables|/Game/Capstone/Blueprints/BP_PlayerCharacter.BP_PlayerCharacter_C|GetWalk%20Speed Player) _status_effect))
  (Utilities|FlowControl|Delay (Variables|Default|GetTime%20Effect%20is%20active))
  (Variables|/Game/Capstone/Blueprints/BP_PlayerCharacter.BP_PlayerCharacter_C|SetSprint%20Speed Player (Variables|/Game/Capstone/Blueprints/BP_PlayerCharacter.BP_PlayerCharacter_C|GetDefault%20Sprint%20Speed Player))
  (Variables|/Game/Capstone/Blueprints/BP_PlayerCharacter.BP_PlayerCharacter_C|SetWalk%20Speed Player (Variables|/Game/Capstone/Blueprints/BP_PlayerCharacter.BP_PlayerCharacter_C|GetDefault%20Walk%20Speed Player))
  (Actor|DestroyActor))

(event EventBeginPlay
  (|CallParentFunction) ; This node is disabled and will not be called.\nDrag off pins to build functionality.
)

(event Collision|EventActorBeginOverlap
  (params (OtherActor :type Actor%20Object%20Reference))
  (|CallParentFunction OtherActor) ; This node is disabled and will not be called.\nDrag off pins to build functionality.
)

(event EventTick
  (params (DeltaSeconds :type Float%20%28single-precision%29))
  (|CallParentFunction DeltaSeconds) ; This node is disabled and will not be called.\nDrag off pins to build functionality.
)

(fn ConstructionScript
  (|CallParentFunction))

(fn UseItem
  (params (Player :type BP%20Player%20Character%20Object%20Reference))
  (CallFunction|ChocolateBoost Player))