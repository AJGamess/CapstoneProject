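; Game mode for a train horror game that tracks objective and floor progress.
; On BeginPlay it resets the completed objective count, sets the maximum from the BP_Objective actors in the level and increments the current floor.
; ObjectiveCompleted increments the count and prints a message, without checking it against the maximum.
; LoadNextLevel opens a random entry from Levels, then increments FloorsCompleted and runs the same reset.
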(event EventBeginPlay
  (CallFunction|ResetValuesforNewFloor))

(event EventTick
  (params (DeltaSeconds :type Float%20%28single-precision%29)))

(fn ConstructionScript)

(fn ObjectiveCompleted
  (Variables|Default|SetObjectiveAmountCompleted (+ (Variables|Default|GetObjectiveAmountCompleted) 1))
  (Development|PrintString "Objective Completed"))

(fn LoadNextLevel
  (bind _levels (Variables|Default|GetLevels))
  (Game|OpenLevel(byName) (Utilities|Array|Get(acopy) _levels (Math|Random|RandomIntegerinRange 0 (- (Utilities|Array|Length _levels) 1))))
  (bind _result (Math|Integer|IncrementInt (Variables|Default|GetFloors%20Completed))
    (:%20%20
      (Variables|Default|SetFloors%20Completed _result)
      (CallFunction|ResetValuesforNewFloor))))

(fn ResetValuesforNewFloor
  (Variables|Default|SetObjectiveAmountCompleted 0)
  (bind _outactors (Actor|GetAllActorsOfClass "/Game/Capstone/Blueprints/BP_Objective.BP_Objective_C"))
  (Variables|Default|SetMaxAmountObjectives (Utilities|Array|Length _outactors))
  (bind _result (Math|Integer|IncrementInt (Variables|Default|GetCurrent%20Floor))
    (:%20%20
      (Variables|Default|SetCurrent%20Floor _result))))